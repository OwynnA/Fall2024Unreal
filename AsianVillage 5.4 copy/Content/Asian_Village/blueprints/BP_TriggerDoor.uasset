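; BP_TriggerDoor is a one-shot trigger volume that puts a door timer on screen when something overlaps its Box.
; The overlap creates a BP_DoorTimer widget for player 0, copies MinutesSet and SecondsSet into its current and reset values, and adds it to the viewport.
; It then disables the Box's collision so it cannot fire again; the overlapping actor is not filtered.
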(event `self.Box.OnComponentBeginOverlap`
  (params (OverlappedComponent :type "PrimitiveComponent Object Reference") (OtherActor :type "Actor Object Reference") (OtherComp :type "PrimitiveComponent Object Reference") (OtherBodyIndex :type Integer) (bFromSweep :type Boolean) (SweepResult :type "HitResult Structure (by ref)"))
  (bind _secondsset (`self.SecondsSet`))
  (bind _minutesset (`self.MinutesSet`))
  (bind _returnvalue (`|CreateWidget` "/Game/Asian_Village/blueprints/BP_DoorTimer.BP_DoorTimer_C" (`GameplayStatics.GetPlayerController` 0)))
  (set `/Game/Asian_Village/blueprints/BP_DoorTimer.SecondsReset` _secondsset _returnvalue)
  (set `/Game/Asian_Village/blueprints/BP_DoorTimer.Seconds` _secondsset _returnvalue)
  (set `/Game/Asian_Village/blueprints/BP_DoorTimer.MInutesReset` _minutesset _returnvalue)
  (set `/Game/Asian_Village/blueprints/BP_DoorTimer.Minutes` _minutesset _returnvalue)
  (`UserWidget.AddToViewport` _returnvalue 0)
  (`PrimitiveComponent.SetCollisionEnabled` (`self.Box`) "NoCollision"))

(fn `UserConstructionScript`)