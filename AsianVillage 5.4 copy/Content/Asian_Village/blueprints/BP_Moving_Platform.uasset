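; Moving platform Blueprint that travels between designer-set relative locations using an InterpToMovement component.
; The construction script builds the control points from Location1 and Location2 and applies Duration, leaving Location3 unused.
; SwitchSpots activates the component, reapplies those points and duration, then immediately deactivates it.
; BeginPlay and the interp-stop event are empty, and the remaining event-graph setup never runs.
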(event `self.ReceiveBeginPlay`)

(event `self.InterpToMovement.OnInterpToStop`
  (params (ImpactResult :type "HitResult Structure (by ref)") (Time :type "Float (single-precision)")))

(fn `SwitchSpots`
  (bind _interptomovement (`self.InterpToMovement`))
  (`ActorComponent.Activate` _interptomovement false)
  (set `InterpToMovementComponent.ControlPoints` (`|MakeArray` (make `InterpControlPoint` (`self.Location1`)) (make `InterpControlPoint` (`self.Location2`)) (struct)) _interptomovement)
  (set `InterpToMovementComponent.Duration` (`self.Duration`) _interptomovement)
  (`ActorComponent.Deactivate` _interptomovement))

(fn `UserConstructionScript`
  (bind _interptomovement (`self.InterpToMovement`))
  (set `InterpToMovementComponent.ControlPoints` (`|MakeArray` (make `InterpControlPoint` (`self.Location1`)) (make `InterpControlPoint` (`self.Location2`)) (struct)) _interptomovement)
  (set `InterpToMovementComponent.Duration` (`self.Duration`) _interptomovement))