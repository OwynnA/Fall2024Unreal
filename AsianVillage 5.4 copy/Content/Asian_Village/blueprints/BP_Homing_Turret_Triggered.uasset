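; Turret actor that, while its IsActive flag is set, turns toward the player character and fires bullets.
; A PawnSensing sighting of BP_ThirdPersonCharacter snaps the actor's rotation to a look-at of that pawn.
; After a short Delay, it spawns BP_Bullet at the Arrow0 component's transform.
; Nothing in this graph sets IsActive.
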(event `self.PawnSensing.OnSeePawn`
  (params (Pawn :type "Pawn Object Reference"))
  (if (`self.isActive`)
    (cast `/Game/ThirdPerson/Blueprints/BP_ThirdPersonCharacter` Pawn)
    (`self.K2_SetActorRotation` (`KismetMathLibrary.FindLookAtRotation` (`self.K2_GetActorLocation`) (`self.K2_GetActorLocation` Pawn)))
    (`KismetSystemLibrary.Delay` 0.2)
    (`|SpawnActorFromClass` "/Game/Asian_Village/blueprints/BP_Bullet.BP_Bullet_C" (`SceneComponent.K2_GetComponentToWorld` (`self.arrow_0`)) "Undefined" "MultiplyWithRoot" null null)))

(fn `UserConstructionScript`)