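; Triggered platform that slides a bridge floor mesh between two relative locations, Location1 and Location2.
; Tick polls a Move flag, flips Position and plays one of two timelines, whose track drives a vector lerp on the mesh.
; Each timeline update clears Move; nothing here sets it.
; The InterpToMovement component is effectively unused: SwitchSpots is empty, its setup code is disconnected, and the stop event does nothing.
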(event `self.ReceiveTick`
  (params (DeltaSeconds :type "Float (single-precision)"))
  (if (`self.move`)
    (if (<= (`self.position`) 0)
      (set `self.position` 1)
      (bind (_direction _newtrack_0) (`Timeline|Position0` :!via `PlayFromStart`)
        (:`Update`
          (`SceneComponent.K2_SetRelativeLocation` (`self.SM_bridge_floor_01`) (`KismetMathLibrary.VLerp` (`self.Location1`) (`self.Location2`) _newtrack_0) false false)
          (set `self.move` false)))
      (else
        (set `self.position` 0)
        (bind (_direction_2 _newtrack_0_2) (`Timeline|Position1` :!via `PlayFromStart`)
          (:`Update`
            (`SceneComponent.K2_SetRelativeLocation` (`self.SM_bridge_floor_01`) (`KismetMathLibrary.VLerp` (`self.Location1`) (`self.Location2`) _newtrack_0_2) false false)
            (set `self.move` false)))))))

(event `self.InterpToMovement.OnInterpToStop`
  (params (ImpactResult :type "HitResult Structure (by ref)") (Time :type "Float (single-precision)")))

(fn `SwitchSpots`)

(fn `UserConstructionScript`)